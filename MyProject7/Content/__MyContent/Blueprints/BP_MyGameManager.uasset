(fn `Get State`
  (returns (NewParam :type "/Game/__MyContent/Blueprints/BP_MyGameStates Enum"))
  (return (`self.Current Game State`)))

(fn `Init`
  (`KismetSystemLibrary.PrintString` "This is the game manager"))

(fn `Set State`
  (params (`New State` :type "/Game/__MyContent/Blueprints/BP_MyGameStates Enum" :default "NewEnumerator4"))
  (if (`|EnumInequality` `New State` (`self.Current Game State`))
    (bind _output_get (set `self.Current Game State` `New State`))
    (switch `/Game/__MyContent/Blueprints/BP_MyGameStates` _output_get
      (:`NewEnumerator1`
        (`KismetSystemLibrary.PrintString` "You won!" true true (struct :`R` 1.0 :`G` 0.923688 :`A` 1.0) 5.0)))))

(fn `UserConstructionScript`)